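; Player character Blueprint that implements hitscan shooting on the Fire input.
; Pressing Fire sets a Firing flag and runs a single debug-drawn line trace from the camera along its forward vector, with the end point nudged downward.
; A hit Enemy has the Damage value subtracted directly from its Life; releasing Fire only clears the flag, and nothing here repeats the shot.
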(event `InputAction|Fire`
  (params (Key :type "Key Structure"))
  (bind _cam (`self.cam`))
  (bind _returnvalue (`SceneComponent.K2_GetComponentLocation` _cam))
  (:`Pressed`
    (set `self.Firing` true)
    (bind (_outhit _returnvalue_2) (`KismetSystemLibrary.LineTraceSingle` :`Start` _returnvalue :`End` (+ _returnvalue (- (* (`SceneComponent.GetForwardVector` _cam) (10000.0 10000.0 10000.0)) (0.0 0.0 100.0))) :`TraceChannel` "TraceTypeQuery3" :`DrawDebugType` "ForDuration"))
    (if _returnvalue_2
      (bind _asenemy (cast `/Game/Blueprints/Enemy` (`.HitActor` (`GameplayStatics.BreakHitResult` _outhit))))
      (set `/Game/Blueprints/Enemy.Life` (- (`/Game/Blueprints/Enemy.Life` _asenemy) (`self.Damage`)) _asenemy)))
  (:`Released`
    (set `self.Firing` false)))

(fn `UserConstructionScript`)